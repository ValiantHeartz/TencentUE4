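; BP_BUllet is a projectile actor that updates the player's score when it hits something.
; On BeginPlay it copies its Velocity variable into the ProjectileMovement component.
; When its Sphere begins an overlap, it casts player character 0 to Ue4ASP_Character, updates Score through a math expression and destroys itself.
; The overlapped actor is never checked, so any overlap scores if that cast succeeds.
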(event OnComponentBeginOverlap(Sphere)
  (params (OverlappedComponent :type Primitive%20Component%20Object%20Reference) (OtherActor :type Actor%20Object%20Reference) (OtherComp :type Primitive%20Component%20Object%20Reference) (OtherBodyIndex :type Integer) (bFromSweep :type Boolean) (SweepResult :type Hit%20Result%20Structure%20%28by%20ref%29))
  (bind _asue_4asp_character (Utilities|Casting|CastToUe4ASP_Character (Game|GetPlayerCharacter 0)))
  (Variables|/Game/AnimStarterPack/Ue4ASP_Character.Ue4ASP_Character_C|SetScore _asue_4asp_character (|(Score+1) (Variables|/Game/AnimStarterPack/Ue4ASP_Character.Ue4ASP_Character_C|GetScore _asue_4asp_character)))
  (Actor|DestroyActor))

(event EventBeginPlay
  (Variables|/Script/Engine.MovementComponent|SetVelocity (Variables|Default|GetProjectileMovement) (Variables|Default|GetVelocity)))

(event Collision|EventActorBeginOverlap
  (params (OtherActor :type Actor%20Object%20Reference)))

(event EventTick
  (params (DeltaSeconds :type Float%20%28single-precision%29)))

(fn ConstructionScript)